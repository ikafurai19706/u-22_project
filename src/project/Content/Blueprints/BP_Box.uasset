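; BP_Box is a physics box that moves under the game's changeable gravity, read from BP_Instance.
; Its construction script sets the PhysicsConstraint to free only the linear axis matching the gravity direction and lock the other two.
; Tick pushes the mesh along that direction with an acceleration force.
; When gravity changes, it destroys itself and spawns a new BP_Box at the mesh's location, so the constraint is rebuilt for the new axis.
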(event `self.ReceiveBeginPlay`
  (bind _asbp_instance (cast `/Game/Blueprints/BP_Instance` (`GameplayStatics.GetGameInstance`)))
  (set `self.As BP Instance` _asbp_instance))

(event `self.ReceiveTick`
  (params (DeltaSeconds :type "Float (single-precision)"))
  (bind _as_bp_instance (`self.As BP Instance`))
  (bind _gravitydirection (`/Game/Blueprints/BP_Instance.gravityDirection` _as_bp_instance))
  (if (`KismetMathLibrary.EqualExactly_VectorVector` (`self.oldGravityDirection`) _gravitydirection)
    (`PrimitiveComponent.AddForce` (`self.SM_Box`) (* (* _gravitydirection (`/Game/Blueprints/BP_Instance.gravityAcceleration` _as_bp_instance)) DeltaSeconds) "None" true)
    (else
      (`PrimitiveComponent.SetPhysicsLinearVelocity` (`self.SM_Box`) (0.0 0.0 0.0) false "None")
      (set `self.oldGravityDirection` _gravitydirection)
      (bind _output_get (set `self.transformLocation` (`SceneComponent.K2_GetComponentLocation` (`self.SM_Box`))))
      (`self.K2_DestroyActor`)
      (`|SpawnActorFromClass` "BP_Box_C" (`KismetMathLibrary.Conv_VectorToTransform` _output_get) "Undefined" "MultiplyWithRoot" null null))))

(fn `UserConstructionScript`
  (bind _physicsconstraint (`self.PhysicsConstraint`))
  (bind _asbp_instance (cast `/Game/Blueprints/BP_Instance` (`GameplayStatics.GetGameInstance`)))
  (bind _output_get (set `self.As BP Instance` _asbp_instance))
  (bind _gravitydirection (`/Game/Blueprints/BP_Instance.gravityDirection` _output_get))
  (set `self.oldGravityDirection` _gravitydirection)
  (if (`KismetMathLibrary.Conv_IntToBool` (`KismetMathLibrary.Abs_Int` (`KismetMathLibrary.Round` (.x _gravitydirection))))
    (`PhysicsConstraintComponent.SetLinearXLimit` _physicsconstraint "LCM_Free" 0.0)
    (`PhysicsConstraintComponent.SetLinearYLimit` _physicsconstraint "LCM_Limited" 0.0)
    (`PhysicsConstraintComponent.SetLinearZLimit` _physicsconstraint "LCM_Limited" 0.0)
    (elif (`KismetMathLibrary.Conv_IntToBool` (`KismetMathLibrary.Abs_Int` (`KismetMathLibrary.Round` (.y _gravitydirection))))
      (`PhysicsConstraintComponent.SetLinearXLimit` _physicsconstraint "LCM_Limited" 0.0)
      (`PhysicsConstraintComponent.SetLinearYLimit` _physicsconstraint "LCM_Free" 0.0)
      (`PhysicsConstraintComponent.SetLinearZLimit` _physicsconstraint "LCM_Limited" 0.0)
      (else
        (`PhysicsConstraintComponent.SetLinearXLimit` _physicsconstraint "LCM_Limited" 0.0)
        (`PhysicsConstraintComponent.SetLinearYLimit` _physicsconstraint "LCM_Limited" 0.0)
        (`PhysicsConstraintComponent.SetLinearZLimit` _physicsconstraint "LCM_Free" 0.0)))))