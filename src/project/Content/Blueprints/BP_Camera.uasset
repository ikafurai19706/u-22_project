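; Camera actor with mouse-driven spring-arm look that reorients itself when the game's gravity direction changes.
; Each tick it applies pitch-clamped mouse rotation and publishes the arm's forward and right vectors to BP_Instance.
; When BP_Instance flags CameraRotating, it adds 90-degree steps from the old/new gravity cross product (absolute values only) to the stored rotation.
; It then eases the root there with ExpoOut and clears the flag.
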(event `self.ReceiveBeginPlay`
  (`self.EnableInput` (`GameplayStatics.GetPlayerController` 0))
  (bind _asbp_instance (cast `/Game/Blueprints/BP_Instance` (`GameplayStatics.GetGameInstance`)))
  (bind _output_get (set `self.As BP Instance` _asbp_instance))
  (set `self.As BP Instance` _output_get))

(event `self.ReceiveTick`
  (params (DeltaSeconds :type "Float (single-precision)"))
  (bind _as_bp_instance (`self.As BP Instance`))
  (bind _returnvalue (+ (.x (`/Game/Blueprints/BP_Instance.V3CameraRotation` (`self.As BP Instance`))) (.x (`KismetMathLibrary.Vector_GetAbs` (* (`KismetMathLibrary.Vector_GetAbs` (`KismetMathLibrary.Cross_VectorVector` (`/Game/Blueprints/BP_Instance.gravityDirection` _as_bp_instance) (`/Game/Blueprints/BP_Instance.old_gravityDirection` _as_bp_instance))) (-90.0 -90.0 -90.0))))))
  (bind _returnvalue_2 (+ (.y (`/Game/Blueprints/BP_Instance.V3CameraRotation` (`self.As BP Instance`))) (.y (`KismetMathLibrary.Vector_GetAbs` (* (`KismetMathLibrary.Vector_GetAbs` (`KismetMathLibrary.Cross_VectorVector` (`/Game/Blueprints/BP_Instance.gravityDirection` _as_bp_instance) (`/Game/Blueprints/BP_Instance.old_gravityDirection` _as_bp_instance))) (-90.0 -90.0 -90.0))))))
  (bind _returnvalue_3 (+ (.z (`/Game/Blueprints/BP_Instance.V3CameraRotation` (`self.As BP Instance`))) (.z (`KismetMathLibrary.Vector_GetAbs` (* (`KismetMathLibrary.Vector_GetAbs` (`KismetMathLibrary.Cross_VectorVector` (`/Game/Blueprints/BP_Instance.gravityDirection` _as_bp_instance) (`/Game/Blueprints/BP_Instance.old_gravityDirection` _as_bp_instance))) (-90.0 -90.0 -90.0))))))
  (`SceneComponent.K2_SetRelativeRotation` (`self.SpringArm`) (`KismetMathLibrary.MakeRotator` (.roll (`SceneComponent.RelativeRotation` (`self.SpringArm`))) (`KismetMathLibrary.FClamp` (+ (.pitch (`SceneComponent.RelativeRotation` (`self.SpringArm`))) (`self.GetInputAxisValue`)) -89.0 89.0) (+ (.yaw (`SceneComponent.RelativeRotation` (`self.SpringArm`))) (`self.GetInputAxisValue`))) false false)
  (set `/Game/Blueprints/BP_Instance.cameraForward` (`SceneComponent.GetForwardVector` (`self.SpringArm`)) (`self.As BP Instance`))
  (set `/Game/Blueprints/BP_Instance.cameraRight` (`SceneComponent.GetRightVector` (`self.SpringArm`)) (`self.As BP Instance`))
  (if (`/Game/Blueprints/BP_Instance.bCameraRotating` (`self.As BP Instance`))
    (if (`self.bRotateSet`)
      (set `self.rotateAlpha` (`KismetMathLibrary.FMin` (+ (`self.rotateAlpha`) (* (`GameplayStatics.GetWorldDeltaSeconds`) (`self.rotateSpeed`))) 1.0))
      (`SceneComponent.K2_SetRelativeRotation` (`self.DefaultSceneRoot`) (`|EaseFunction` "ExpoOut" (`self.rotateAlpha`) (`self.rootRotation`) (`self.targetRotation`)) false false)
      (if (>= (`self.rotateAlpha`) 1.0)
        (set `/Game/Blueprints/BP_Instance.bCameraRotating` false (`self.As BP Instance`))
        (set `self.bRotateSet` false)
        (set `self.rotateAlpha` 0.0))
      (else
        (set `self.bRotateSet` true)
        (set `self.rootRotation` (`SceneComponent.GetSocketRotation` (`self.DefaultSceneRoot`) "None"))
        (set `self.targetRotation` (`KismetMathLibrary.MakeRotator` _returnvalue _returnvalue_2 _returnvalue_3))
        (set `/Game/Blueprints/BP_Instance.V3CameraRotation` (`KismetMathLibrary.MakeVector` _returnvalue _returnvalue_2 _returnvalue_3) (`self.As BP Instance`))))))

(fn `UserConstructionScript`)