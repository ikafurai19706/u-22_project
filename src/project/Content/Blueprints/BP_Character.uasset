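; Physics-driven player character for a game with switchable gravity, reading gravity and camera state from BP_Instance.
; Tick applies gravity, clamps speed on the perpendicular plane, zeroes velocity when gravity changes, and prints a debug counter.
; Axis inputs push the mesh along camera directions masked to the movement plane, except during camera rotation.
; During rotation it derives a gravity-flip target, then replaces itself each tick with an eased-rotation respawn; the rotation-reset branch is unwired.
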(event `self.ReceiveBeginPlay`
  (bind _asbp_instance (cast `/Game/Blueprints/BP_Instance` (`GameplayStatics.GetGameInstance`)))
  (set `self.As BP Instance` _asbp_instance)
  (`self.EnableInput` (`GameplayStatics.GetPlayerController` 0)))

(event `self.ReceiveTick`
  (params (DeltaSeconds :type "Float (single-precision)"))
  (bind _as_bp_instance (`self.As BP Instance`))
  (bind _gravitydirection (`/Game/Blueprints/BP_Instance.gravityDirection` _as_bp_instance))
  (`|ExecutionSequence`
    (:`then_0`
      (if (`/Game/Blueprints/BP_Instance.bCameraRotating` (`self.As BP Instance`))
        (if (`self.bRotateSet`)
          (set `self.rotateAlpha` (`KismetMathLibrary.FMin` (+ (`self.rotateAlpha`) (* (`GameplayStatics.GetWorldDeltaSeconds`) (`self.rotateSpeed`))) 1.0))
          (bind _output_get (set `self.TransformLocation_Character` (`SceneComponent.K2_GetComponentLocation` (`self.SM_Character`))))
          (`|SpawnActorFromClass` "BP_Character_C" (`KismetMathLibrary.MakeTransform` _output_get (`|EaseFunction` "ExpoOut" (`self.rotateAlpha`) (`self.rootRotation`) (`self.targetRotation`))) "AdjustIfPossibleButAlwaysSpawn" "MultiplyWithRoot" null null)
          (`self.K2_DestroyActor`)
          (else
            (bind _newparam1 (`self.新規関数` (`self.targetRotation`)))
            (set `self.bRotateSet` true)
            (set `self.rootRotation` (`SceneComponent.GetSocketRotation` (`self.SM_Character`) "None"))
            (set `self.targetRotation` _newparam1)))))
    (:`then_1`
      (bind _output_get_2 (set `self.test` (+ (`self.test`) 1)))
      (`KismetSystemLibrary.PrintString` (`KismetStringLibrary.Conv_IntToString` _output_get_2)))
    (:`then_2`
      (if (`KismetMathLibrary.EqualExactly_VectorVector` (`self.oldGravityDirection`) _gravitydirection)
        (`PrimitiveComponent.AddForce` (`self.SM_Character`) (* (* _gravitydirection (`/Game/Blueprints/BP_Instance.gravityAcceleration` _as_bp_instance)) DeltaSeconds) "None" true)
        (bind _returnvalue (`PrimitiveComponent.GetPhysicsLinearVelocity` (`self.SM_Character`) "None"))
        (if (`KismetMathLibrary.Conv_IntToBool` (`KismetMathLibrary.Abs_Int` (`KismetMathLibrary.Round` (.x (`/Game/Blueprints/BP_Instance.gravityDirection` (`self.As BP Instance`))))))
          (bind _x (.x _returnvalue))
          (bind _y (.y _returnvalue))
          (bind _z (.z _returnvalue))
          (bind _returnvalue_2 (`KismetMathLibrary.MakeVector2D` _y _z))
          (if (> (`KismetMathLibrary.VSize2D` _returnvalue_2) (`self.maxSpeed`))
            (bind (_x_2 _y_2) (`KismetMathLibrary.BreakVector2D` (* (`KismetMathLibrary.Normal2D` _returnvalue_2) (`self.maxSpeed`))))
            (`PrimitiveComponent.SetPhysicsLinearVelocity` (`self.SM_Character`) (`KismetMathLibrary.MakeVector` (.x _returnvalue) _x_2 _y_2) false "None"))
          (elif (`KismetMathLibrary.Conv_IntToBool` (`KismetMathLibrary.Abs_Int` (`KismetMathLibrary.Round` (.y (`/Game/Blueprints/BP_Instance.gravityDirection` (`self.As BP Instance`))))))
            (bind _returnvalue_3 (`KismetMathLibrary.MakeVector2D` _x _z))
            (if (> (`KismetMathLibrary.VSize2D` _returnvalue_3) (`self.maxSpeed`))
              (bind (_x_3 _y_3) (`KismetMathLibrary.BreakVector2D` (* (`KismetMathLibrary.Normal2D` _returnvalue_3) (`self.maxSpeed`))))
              (`PrimitiveComponent.SetPhysicsLinearVelocity` (`self.SM_Character`) (`KismetMathLibrary.MakeVector` _x_3 (.y _returnvalue) _y_3) false "None"))
            (else
              (bind _returnvalue_4 (`KismetMathLibrary.MakeVector2D` _x _y))
              (if (> (`KismetMathLibrary.VSize2D` _returnvalue_4) (`self.maxSpeed`))
                (bind (_x_4 _y_4) (`KismetMathLibrary.BreakVector2D` (* (`KismetMathLibrary.Normal2D` _returnvalue_4) (`self.maxSpeed`))))
                (`PrimitiveComponent.SetPhysicsLinearVelocity` (`self.SM_Character`) (`KismetMathLibrary.MakeVector` _x_4 _y_4 (.z _returnvalue)) false "None")))))
        (else
          (`PrimitiveComponent.SetPhysicsLinearVelocity` (`self.SM_Character`) (0.0 0.0 0.0) false "None")
          (set `self.oldGravityDirection` _gravitydirection))))))

(event `InputAxis|前後`
  (params (AxisValue :type "Float (single-precision)"))
  (`PrimitiveComponent.AddForce` (`self.SM_Character`) (* (`KismetMathLibrary.Normal` (* (`/Game/Blueprints/BP_Instance.cameraForward` (`self.As BP Instance`)) (`/Game/Blueprints/BP_Instance.移動する面` (`self.As BP Instance`)))) (* (* AxisValue 5000.0) (not (`/Game/Blueprints/BP_Instance.bCameraRotating` (`self.As BP Instance`))))) "None" true))

(event `InputAxis|左右`
  (params (AxisValue :type "Float (single-precision)"))
  (`PrimitiveComponent.AddForce` (`self.SM_Character`) (* (`KismetMathLibrary.Normal` (* (`/Game/Blueprints/BP_Instance.移動する面` (`self.As BP Instance`)) (`/Game/Blueprints/BP_Instance.cameraRight` (`self.As BP Instance`)))) (* (* AxisValue 5000.0) (not (`/Game/Blueprints/BP_Instance.bCameraRotating` (`self.As BP Instance`))))) "None" true))

(fn `UserConstructionScript`
  (bind _asbp_instance (cast `/Game/Blueprints/BP_Instance` (`GameplayStatics.GetGameInstance`)))
  (set `self.As BP Instance` _asbp_instance))

(fn `新規関数`
  (params (NewParam :type "Rotator Structure"))
  (returns (NewParam1 :type "Rotator Structure"))
  (bind _as_bp_instance (`self.As BP Instance`))
  (bind _returnvalue (`KismetMathLibrary.Cross_VectorVector` (`/Game/Blueprints/BP_Instance.gravityDirection` _as_bp_instance) (`/Game/Blueprints/BP_Instance.old_gravityDirection` _as_bp_instance)))
  (if (== (`KismetMathLibrary.Vector_GetAbsMax` _returnvalue) 0.0)
    (bind _newparam1 (`self.新規関数_0` (`/Game/Blueprints/BP_Instance.cameraForward` (`self.As BP Instance`))))
    (return (`KismetMathLibrary.ComposeRotators` NewParam (`KismetMathLibrary.MakeRotator` (.x (* _newparam1 (180.0 180.0 180.0))) (.y (* _newparam1 (180.0 180.0 180.0))) (.z (* _newparam1 (180.0 180.0 180.0))))))
    (else
      (return (`KismetMathLibrary.ComposeRotators` NewParam (`KismetMathLibrary.MakeRotator` (.x (* _returnvalue (90.0 90.0 -90.0))) (.y (* _returnvalue (90.0 90.0 -90.0))) (.z (* _returnvalue (90.0 90.0 -90.0)))))))))

(fn `新規関数_0`
  (params (NewParam :type "Vector Structure"))
  (returns (NewParam1 :type "Vector Structure"))
  (bind `_移動する面` (`/Game/Blueprints/BP_Instance.移動する面` (`self.As BP Instance`)))
  (bind _returnvalue (* NewParam `_移動する面` (1.0 0.0 0.0)))
  (bind _returnvalue_2 (* `_移動する面` NewParam (0.0 1.0 0.0)))
  (bind _returnvalue_3 (* `_移動する面` NewParam (0.0 0.0 1.0)))
  (bind _returnvalue_4 (`KismetMathLibrary.VSizeSquared` _returnvalue))
  (bind _returnvalue_5 (`KismetMathLibrary.VSizeSquared` _returnvalue_2))
  (bind _returnvalue_6 (`KismetMathLibrary.VSizeSquared` _returnvalue_3))
  (if (and (>= _returnvalue_4 _returnvalue_5) (>= _returnvalue_4 _returnvalue_6))
    (return (`KismetMathLibrary.Normal` _returnvalue))
    (elif (>= _returnvalue_5 _returnvalue_6)
      (return (`KismetMathLibrary.Normal` _returnvalue_2))
      (else
        (return (`KismetMathLibrary.Normal` _returnvalue_3))))))