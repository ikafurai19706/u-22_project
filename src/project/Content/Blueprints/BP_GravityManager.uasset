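; Gravity manager that lets the player rotate world gravity with the arrow keys or flip it with G.
; Arrows snap gravity to the dominant world axis of the camera's forward or right vector, masked to the plane perpendicular to current gravity.
; Tick refreshes that plane mask in BP_Instance, the GameInstance holding the shared state.
; Each change sets CameraRotating and blocks further input for one second before saving OldGravityDirection.
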(event `Key|Up`
  (params (Key :type "Key Structure"))
  (bind _cameraforward (`/Game/Blueprints/BP_Instance.cameraForward` (`self.As BP Instance`)))
  (bind `_移動する面` (`/Game/Blueprints/BP_Instance.移動する面` (`self.As BP Instance`)))
  (bind _returnvalue (* `_移動する面` _cameraforward (0.0 0.0 1.0)))
  (bind _returnvalue_2 (* _cameraforward `_移動する面` (1.0 0.0 0.0)))
  (bind _returnvalue_3 (* `_移動する面` _cameraforward (0.0 1.0 0.0)))
  (bind _returnvalue_4 (`KismetMathLibrary.VSizeSquared` _returnvalue_2))
  (bind _returnvalue_5 (`KismetMathLibrary.VSizeSquared` _returnvalue_3))
  (bind _returnvalue_6 (`KismetMathLibrary.VSizeSquared` _returnvalue))
  ;[1 1 1 1 100] 重力の向き変更
  (:`Pressed`
    (if (not (`self.bPressed`))
      (set `self.bPressed` true)
      ;;[1 0.7055 0.6756] それぞれ大きさ比較して最大の向きに更新してる
      (if (and (>= _returnvalue_4 _returnvalue_5) (>= _returnvalue_4 _returnvalue_6))
        (`self.ApplyDirection` _returnvalue_2)
        (elif (>= _returnvalue_5 _returnvalue_6)
          (`self.ApplyDirection` _returnvalue_3)
          (else
            (`self.ApplyDirection` _returnvalue)))))))

(event `self.ReceiveBeginPlay`
  (bind _asbp_instance (cast `/Game/Blueprints/BP_Instance` (`GameplayStatics.GetGameInstance`)))
  (set `self.As BP Instance` _asbp_instance)
  (`self.EnableInput` (`GameplayStatics.GetPlayerController` 0))
  (set `/Game/Blueprints/BP_Instance.移動する面` (1.0 1.0 0.0) (`self.As BP Instance`)))

(event `self.ReceiveTick`
  (params (DeltaSeconds :type "Float (single-precision)"))
  (set `/Game/Blueprints/BP_Instance.移動する面` (- (1.0 1.0 1.0) (`KismetMathLibrary.Vector_GetAbs` (`/Game/Blueprints/BP_Instance.gravityDirection` (`self.As BP Instance`)))) (`self.As BP Instance`)))

(event `Key|Down`
  (params (Key :type "Key Structure"))
  (bind _cameraforward (`/Game/Blueprints/BP_Instance.cameraForward` (`self.As BP Instance`)))
  (bind `_移動する面` (`/Game/Blueprints/BP_Instance.移動する面` (`self.As BP Instance`)))
  (bind _returnvalue (* _cameraforward `_移動する面` (1.0 0.0 0.0)))
  (bind _returnvalue_2 (* `_移動する面` _cameraforward (0.0 1.0 0.0)))
  (bind _returnvalue_3 (* `_移動する面` _cameraforward (0.0 0.0 1.0)))
  (bind _returnvalue_4 (`KismetMathLibrary.VSizeSquared` _returnvalue))
  (bind _returnvalue_5 (`KismetMathLibrary.VSizeSquared` _returnvalue_2))
  (bind _returnvalue_6 (`KismetMathLibrary.VSizeSquared` _returnvalue_3))
  ;[1 1 1 1 100] 重力の向き変更
  (:`Pressed`
    (if (not (`self.bPressed`))
      (set `self.bPressed` true)
      (if (and (>= _returnvalue_4 _returnvalue_5) (>= _returnvalue_4 _returnvalue_6))
        (bind _output_get (set `/Game/Blueprints/BP_Instance.gravityDirection` (* (`KismetMathLibrary.Normal` _returnvalue) (-1.0 -1.0 -1.0)) (`self.As BP Instance`)))
        (set `/Game/Blueprints/BP_Instance.bCameraRotating` true (`self.As BP Instance`))
        (`KismetSystemLibrary.Delay` 1.0)
        (set `self.bPressed` false)
        (set `/Game/Blueprints/BP_Instance.old_gravityDirection` _output_get (`self.As BP Instance`))
        (elif (>= _returnvalue_5 _returnvalue_6)
          (bind _output_get_2 (set `/Game/Blueprints/BP_Instance.gravityDirection` (* (`KismetMathLibrary.Normal` _returnvalue_2) (-1.0 -1.0 -1.0)) (`self.As BP Instance`)))
          (set `/Game/Blueprints/BP_Instance.bCameraRotating` true (`self.As BP Instance`))
          (`KismetSystemLibrary.Delay` 1.0)
          (set `self.bPressed` false)
          (set `/Game/Blueprints/BP_Instance.old_gravityDirection` _output_get_2 (`self.As BP Instance`))
          (else
            (bind _output_get_3 (set `/Game/Blueprints/BP_Instance.gravityDirection` (* (`KismetMathLibrary.Normal` _returnvalue_3) (-1.0 -1.0 -1.0)) (`self.As BP Instance`)))
            (set `/Game/Blueprints/BP_Instance.bCameraRotating` true (`self.As BP Instance`))
            (`KismetSystemLibrary.Delay` 1.0)
            (set `self.bPressed` false)
            (set `/Game/Blueprints/BP_Instance.old_gravityDirection` _output_get_3 (`self.As BP Instance`))))))))

(event `Key|Right`
  (params (Key :type "Key Structure"))
  (bind `_移動する面` (`/Game/Blueprints/BP_Instance.移動する面` (`self.As BP Instance`)))
  (bind _cameraright (`/Game/Blueprints/BP_Instance.cameraRight` (`self.As BP Instance`)))
  (bind _returnvalue (* _cameraright `_移動する面` (1.0 0.0 0.0)))
  (bind _returnvalue_2 (* `_移動する面` _cameraright (0.0 1.0 0.0)))
  (bind _returnvalue_3 (* `_移動する面` (0.0 0.0 1.0) _cameraright))
  (bind _returnvalue_4 (`KismetMathLibrary.VSizeSquared` _returnvalue))
  (bind _returnvalue_5 (`KismetMathLibrary.VSizeSquared` _returnvalue_2))
  (bind _returnvalue_6 (`KismetMathLibrary.VSizeSquared` _returnvalue_3))
  ;[1 1 1 1 100] 重力の向き変更
  (:`Pressed`
    (if (not (`self.bPressed`))
      (set `self.bPressed` true)
      (if (and (>= _returnvalue_4 _returnvalue_5) (>= _returnvalue_4 _returnvalue_6))
        (bind _output_get (set `/Game/Blueprints/BP_Instance.gravityDirection` (`KismetMathLibrary.Normal` _returnvalue) (`self.As BP Instance`)))
        (set `/Game/Blueprints/BP_Instance.bCameraRotating` true (`self.As BP Instance`))
        (`KismetSystemLibrary.Delay` 1.0)
        (set `self.bPressed` false)
        (set `/Game/Blueprints/BP_Instance.old_gravityDirection` _output_get (`self.As BP Instance`))
        (elif (>= _returnvalue_5 _returnvalue_6)
          (bind _output_get_2 (set `/Game/Blueprints/BP_Instance.gravityDirection` (`KismetMathLibrary.Normal` _returnvalue_2) (`self.As BP Instance`)))
          (set `/Game/Blueprints/BP_Instance.bCameraRotating` true (`self.As BP Instance`))
          (`KismetSystemLibrary.Delay` 1.0)
          (set `self.bPressed` false)
          (set `/Game/Blueprints/BP_Instance.old_gravityDirection` _output_get_2 (`self.As BP Instance`))
          (else
            (bind _output_get_3 (set `/Game/Blueprints/BP_Instance.gravityDirection` (`KismetMathLibrary.Normal` _returnvalue_3) (`self.As BP Instance`)))
            (set `/Game/Blueprints/BP_Instance.bCameraRotating` true (`self.As BP Instance`))
            (`KismetSystemLibrary.Delay` 1.0)
            (set `self.bPressed` false)
            (set `/Game/Blueprints/BP_Instance.old_gravityDirection` _output_get_3 (`self.As BP Instance`))))))))

(event `Key|Left`
  (params (Key :type "Key Structure"))
  (bind `_移動する面` (`/Game/Blueprints/BP_Instance.移動する面` (`self.As BP Instance`)))
  (bind _cameraright (`/Game/Blueprints/BP_Instance.cameraRight` (`self.As BP Instance`)))
  (bind _returnvalue (* _cameraright `_移動する面` (1.0 0.0 0.0)))
  (bind _returnvalue_2 (* `_移動する面` _cameraright (0.0 1.0 0.0)))
  (bind _returnvalue_3 (* `_移動する面` _cameraright (0.0 0.0 1.0)))
  (bind _returnvalue_4 (`KismetMathLibrary.VSizeSquared` _returnvalue_3))
  (bind _returnvalue_5 (`KismetMathLibrary.VSizeSquared` _returnvalue))
  (bind _returnvalue_6 (`KismetMathLibrary.VSizeSquared` _returnvalue_2))
  ;[1 1 1 1 100] 重力の向き変更
  (:`Pressed`
    (if (not (`self.bPressed`))
      (set `self.bPressed` true)
      (if (and (>= _returnvalue_5 _returnvalue_6) (>= _returnvalue_5 _returnvalue_4))
        (bind _output_get (set `/Game/Blueprints/BP_Instance.gravityDirection` (* (`KismetMathLibrary.Normal` _returnvalue) (-1.0 -1.0 -1.0)) (`self.As BP Instance`)))
        (set `/Game/Blueprints/BP_Instance.bCameraRotating` true (`self.As BP Instance`))
        (`KismetSystemLibrary.Delay` 1.0)
        (set `self.bPressed` false)
        (set `/Game/Blueprints/BP_Instance.old_gravityDirection` _output_get (`self.As BP Instance`))
        (elif (>= _returnvalue_6 _returnvalue_4)
          (bind _output_get_2 (set `/Game/Blueprints/BP_Instance.gravityDirection` (* (`KismetMathLibrary.Normal` _returnvalue_2) (-1.0 -1.0 -1.0)) (`self.As BP Instance`)))
          (set `/Game/Blueprints/BP_Instance.bCameraRotating` true (`self.As BP Instance`))
          (`KismetSystemLibrary.Delay` 1.0)
          (set `self.bPressed` false)
          (set `/Game/Blueprints/BP_Instance.old_gravityDirection` _output_get_2 (`self.As BP Instance`))
          (else
            (bind _output_get_3 (set `/Game/Blueprints/BP_Instance.gravityDirection` (* (`KismetMathLibrary.Normal` _returnvalue_3) (-1.0 -1.0 -1.0)) (`self.As BP Instance`)))
            (set `/Game/Blueprints/BP_Instance.bCameraRotating` true (`self.As BP Instance`))
            (`KismetSystemLibrary.Delay` 1.0)
            (set `self.bPressed` false)
            (set `/Game/Blueprints/BP_Instance.old_gravityDirection` _output_get_3 (`self.As BP Instance`))))))))

(event `Key|G`
  (params (Key :type "Key Structure"))
  ;[1 1 1 1 100] 重力の向き変更
  ;;[1 0.6627 0.3412] 重力反転だから×-1
  (:`Pressed`
    (if (not (`self.bPressed`))
      (set `self.bPressed` true)
      (bind _output_get (set `/Game/Blueprints/BP_Instance.gravityDirection` (* (`/Game/Blueprints/BP_Instance.gravityDirection` (`self.As BP Instance`)) (-1.0 -1.0 -1.0)) (`self.As BP Instance`)))
      (set `/Game/Blueprints/BP_Instance.bCameraRotating` true (`self.As BP Instance`))
      (`KismetSystemLibrary.Delay` 1.0)
      (set `self.bPressed` false)
      (set `/Game/Blueprints/BP_Instance.old_gravityDirection` _output_get (`self.As BP Instance`)))))

(fn `UserConstructionScript`)