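; MyCharacter is a character Blueprint that moves relative to the camera from the 前後 (forward/back) and 左右 (left/right) input axes.
; BeginPlay caches the BP_Instance game instance and sets Speed.
; Each axis event reads CameraForward or CameraRight from that instance, flattens it to the horizontal plane, normalizes it, multiplies by Speed, and passes it to AddMovementInput scaled by the axis value.
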(event `self.ReceiveBeginPlay`
  (bind _asbp_instance (cast `/Game/Blueprints/BP_Instance` (`GameplayStatics.GetGameInstance`)))
  (set `self.As BP Instance` _asbp_instance)
  (set `self.speed` 100.0))

(event `self.ReceiveTick`
  (params (DeltaSeconds :type "Float (single-precision)")))

(event `InputAxis|前後`
  (params (AxisValue :type "Float (single-precision)"))
  (`self.AddMovementInput` (* (`KismetMathLibrary.Normal` (`KismetMathLibrary.MakeVector` (* (.x (`/Game/Blueprints/BP_Instance.cameraForward` (`self.As BP Instance`))) 1.0) (* (.y (`/Game/Blueprints/BP_Instance.cameraForward` (`self.As BP Instance`))) 1.0) (* (.z (`/Game/Blueprints/BP_Instance.cameraForward` (`self.As BP Instance`))) 0.0))) (`self.speed`)) AxisValue))

(event `InputAxis|左右`
  (params (AxisValue :type "Float (single-precision)"))
  (`self.AddMovementInput` (* (`KismetMathLibrary.Normal` (`KismetMathLibrary.MakeVector` (* (.x (`/Game/Blueprints/BP_Instance.cameraRight` (`self.As BP Instance`))) 1.0) (* (.y (`/Game/Blueprints/BP_Instance.cameraRight` (`self.As BP Instance`))) 1.0) (* (.z (`/Game/Blueprints/BP_Instance.cameraRight` (`self.As BP Instance`))) 0.0))) (`self.speed`)) AxisValue))

(fn `UserConstructionScript`)